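; BP_Battery is a battery pickup that adds to the player's battery count.
; On BeginPlay it finds and stores the BP_Player1 actor through GetActorOfClass.
; InteractText prints a "Take" prompt as a debug string.
; InteractEvent prints "Took", increments BatteryNumber on the stored player and destroys the pickup.
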(event EventBeginPlay
  (bind _returnvalue (Actor|GetActorOfClass "/Game/Player/Blueprints/BP_Player1.BP_Player1_C"))
  (Variables|Default|SetPlayer _returnvalue))

(event EventInteractText
  (Development|PrintString "Take"))

(event EventInteractEvent
  (bind _player (Variables|Default|GetPlayer))
  (Development|PrintString "Took")
  (Variables|/Game/Player/Blueprints/BP_Player1.BP_Player1_C|SetBatteryNumber _player (+ (Variables|/Game/Player/Blueprints/BP_Player1.BP_Player1_C|GetBatteryNumber _player) 1))
  (Actor|DestroyActor))

(fn ConstructionScript)