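; BP_Light is a light actor that can be toggled on and off through its ToggleLight event.
; Each tick, while the light is visible, it gathers enemies of class BPP_Enemy overlapping its box volume.
; For each one it only prints a debug message, so no gameplay effect on enemies is implemented.
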(event Custom|ToggleLight
  (Rendering|ToggleVisibility (Variables|Default|GetLight) false))

(event EventTick
  (params (DeltaSeconds :type Float%20%28single-precision%29))
  (if (Rendering|IsVisible (Variables|Default|GetLight))
    (for _array_element (Collision|GetOverlappingActors (Variables|Default|GetBox) "/Game/Enemies/Blueprints/BPP_Enemy.BPP_Enemy_C" :!class /Script/Engine.PrimitiveComponent)
      (Utilities|Casting|CastToBPP_Enemy _array_element)
      (Development|PrintString "Hello"))))

(fn ConstructionScript)