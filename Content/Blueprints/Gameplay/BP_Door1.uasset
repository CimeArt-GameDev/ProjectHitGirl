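; BP_Door1 is an interactable door that swings open and closed around its yaw axis.
; InteractEvent flips the Opened flag and plays or reverses DoorTimeLine, whose Rotation track drives the Door component's relative rotation.
; InteractText prints an Open or Close label based on the current state.
; The construction script pre-rotates the door when Opened is set, so instances can start open in the level.
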(event EventInteractText
  (if (Variables|Default|GetOpened)
    (Development|PrintString "Close")
    (else
      (Development|PrintString "Open"))))

(event EventInteractEvent
  (if (Variables|Default|GetOpened)
    (Variables|Default|SetOpened false)
    (bind _rotation (Timeline|DoorTimeLine Reverse)
      (:Update
        (Transformation|SetRelativeRotation (Variables|Default|GetDoor) (Math|Rotator|MakeRotator 0.0 0.0 _rotation) false false)))
    (else
      (Variables|Default|SetOpened true)
      (Timeline|DoorTimeLine Play))))

(fn ConstructionScript
  (if (Variables|Default|GetOpened)
    (Transformation|SetRelativeRotation (Variables|Default|GetDoor) "0,110.000000, 0" false false)))