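; BP_Door2 is an interactable swinging door that also opens automatically for enemies.
; Interaction toggles Opened and plays or reverses a timeline driving the door's yaw, with InteractText printing "Open" or "Close".
; Tick polls a Box for overlapping BPP_Enemy actors to open a closed door.
; Collision is disabled during the swing and restored afterward, and the construction script pre-rotates doors that start open.
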(event Custom|OpenDoor
  (bind _door (Variables|Default|GetDoor))
  (Collision|SetCollisionEnabled (Variables|Default|GetDoor) "NoCollision")
  (Variables|Default|SetOpened true)
  (bind _rotation (Timeline|DoorTimeLine Play)
    (:Update
      (Transformation|SetRelativeRotation _door (Math|Rotator|MakeRotator 0.0 0.0 _rotation) false false))
    (:Finished
      (Collision|SetCollisionEnabled _door "QueryAndPhysics"))))

(event EventTick
  (params (DeltaSeconds :type Float%20%28single-precision%29))
  (if (and (> (Utilities|Array|Length (Collision|GetOverlappingActors (Variables|Default|GetBox) "/Game/Enemies/Blueprints/BPP_Enemy.BPP_Enemy_C" :!class /Script/Engine.PrimitiveComponent)) 0) (not (Variables|Default|GetOpened)))
    (CallFunction|OpenDoor)))

(event EventInteractText
  (if (Variables|Default|GetOpened)
    (Development|PrintString "Close")
    (else
      (Development|PrintString "Open"))))

(event EventInteractEvent
  (bind _door (Variables|Default|GetDoor))
  (Collision|SetCollisionEnabled (Variables|Default|GetDoor) "NoCollision")
  (if (Variables|Default|GetOpened)
    (Variables|Default|SetOpened false)
    (bind _rotation (Timeline|DoorTimeLine Reverse)
      (:Update
        (Transformation|SetRelativeRotation _door (Math|Rotator|MakeRotator 0.0 0.0 _rotation) false false))
      (:Finished
        (Collision|SetCollisionEnabled _door "QueryAndPhysics")))
    (else
      (Variables|Default|SetOpened true)
      (Timeline|DoorTimeLine Play))))

(fn ConstructionScript
  (if (Variables|Default|GetOpened)
    (Transformation|SetRelativeRotation (Variables|Default|GetDoor) "0,110.000000, 0" false false)))