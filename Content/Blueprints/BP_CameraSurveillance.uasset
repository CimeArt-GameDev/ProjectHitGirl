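; BP_CameraSurveillance is a surveillance camera actor whose view rotation is set from angle values.
; Its AngleVision event stores the child actor cast to Chameleon, then sets the camera's world roll and pitch from clamped AngleX and AngleY, keeping yaw.
; The clamp bounds are reversed, with the minimum above the maximum.
; ChangeCamera is empty, and the post-process and possession nodes are unconnected.
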(event Custom|AngleVision
  (bind _camera (Variables|Default|GetCamera))
  (Variables|Default|Setchamelon (.AsChameleon (Utilities|Casting|CastToChameleon (Variables|/Script/Engine.ChildActorComponent|GetChildActor (Variables|Default|GetChildActor)))))
  (Transformation|SetWorldRotation _camera (Math|Rotator|MakeRotator (Math|Float|ClampAngle (Variables|Default|GetAngle%20X) 8e+01 -8e+01) (Math|Float|ClampAngle (Variables|Default|GetAngle%20Y) 8e+01 -8e+01) (.yaw (Transformation|GetWorldRotation _camera))) false false))

(fn ConstructionScript)

(fn ChangeCamera)