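; PC_Player2 is a player controller that lets the second player cycle through surveillance cameras placed in the level.
; On BeginPlay it gathers all BP_CameraSurveillance actors into an array and possesses the first one.
; The ChangeCameraRight and ChangeCameraLeft inputs step the index with wraparound, then a PossesCamera event unpossesses the current camera and possesses the newly selected one.
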(event Custom|PossesCamera
  (params (Camera :type BP%20Camera%20Surveillance%20Object%20Reference))
  ;[1 1 1] Event Posses
  (Pawn|UnPossess)
  (Pawn|Possess Camera))

(event EventBeginPlay
  ;[1 1 1] First Posses
  (bind _outactors (Actor|GetAllActorsOfClass "/Game/Blueprints/Camera/BP_CameraSurveillance.BP_CameraSurveillance_C"))
  (bind _output_get (Variables|Default|SetCam _outactors))
  (CallFunction|PossesCamera (Utilities|Array|Get(acopy) _output_get)))

(event Input|ActionEvents|InputActionChangeCameraLeft
  (params (Key :type Key%20Structure :default "None"))
  ;[1 1 1] Changement de camera
  (:Pressed
    (bind _output_get (Variables|Default|SetIndexCamera (select (<= (Variables|Default|GetIndexCamera) 0) (Utilities|Array|LastIndex (Variables|Default|GetCam)) (- (Variables|Default|GetIndexCamera) 1))))
    (CallFunction|PossesCamera (Utilities|Array|Get(acopy) (Variables|Default|GetCam) _output_get))))

(event Input|ActionEvents|InputActionChangeCameraRight
  (params (Key :type Key%20Structure :default "None"))
  ;[1 1 1] Changement de camera
  (:Pressed
    (bind _output_get (Variables|Default|SetIndexCamera (select (>= (Variables|Default|GetIndexCamera) (Utilities|Array|LastIndex (Variables|Default|GetCam))) 0 (+ (Variables|Default|GetIndexCamera) 1))))
    (CallFunction|PossesCamera (Utilities|Array|Get(acopy) (Variables|Default|GetCam) _output_get))))

(fn ConstructionScript)