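; BP_PlayerState switches the first player controller between four camera pawns (CS1–CS4), possessing CS1 at BeginPlay.
; Left and right input actions validate all four references, then increment or decrement Switch respectively, guarded by checks against 0 and 3.
; ChangeCamera maps Switch to CS2, CS3 or CS4, with no branch back to CS1, and calls UnPossess immediately after each Possess.
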(event Custom|ChangeCamera
  (bind _returnvalue (Game|GetPlayerController 0))
  (switch int (Variables|Default|GetSwitch)
    (:0
      (Pawn|Possess _returnvalue (Variables|Default|GetCS2)))
    (:1
      (Pawn|Possess (Game|GetPlayerController 0) (Variables|Default|GetCS3)))
    (:2
      (Pawn|Possess (Game|GetPlayerController 0) (Variables|Default|GetCS4))))
  (Pawn|UnPossess _returnvalue))

(event Custom|ChangeLeft
  (if (!= (Variables|Default|GetSwitch) 0)
    (Math|Integer|IncrementInt (Variables|Default|GetSwitch)
      (:%20%20
        (CallFunction|ChangeCamera)))))

(event Custom|ChangeRight
  (if (!= (Variables|Default|GetSwitch) 3)
    (Math|Integer|DecrementInt (Variables|Default|GetSwitch)
      (:%20%20
        (CallFunction|ChangeCamera)))))

(event EventBeginPlay
  (Pawn|Possess (Game|GetPlayerController 0) (Variables|Default|GetCS1)))

(event Input|ActionEvents|InputActionChangeCameraLeft
  (params (Key :type Key%20Structure :default "None"))
  (:Pressed
    (Development|PrintString "Left")
    (Utilities|IsValid (Variables|Default|GetCS1)
      (:Is%20Valid
        (Utilities|IsValid (Variables|Default|GetCS2)
          (:Is%20Valid
            (Utilities|IsValid (Variables|Default|GetCS3)
              (:Is%20Valid
                (Utilities|IsValid (Variables|Default|GetCS4)
                  (:Is%20Valid
                    (CallFunction|ChangeLeft)))))))))))

(event Input|ActionEvents|InputActionChangeCameraRight
  (params (Key :type Key%20Structure :default "None"))
  (:Pressed
    (Development|PrintString "Right")
    (Utilities|IsValid (Variables|Default|GetCS1)
      (:Is%20Valid
        (Utilities|IsValid (Variables|Default|GetCS2)
          (:Is%20Valid
            (Utilities|IsValid (Variables|Default|GetCS3)
              (:Is%20Valid
                (Utilities|IsValid (Variables|Default|GetCS4)
                  (:Is%20Valid
                    (CallFunction|ChangeRight)))))))))))

(fn ConstructionScript)