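; BP_CameraSurveillance is a surveillance camera Blueprint, currently an unfinished stub with no working behavior.
; BeginPlay calls the AngleVision event, which is empty, and the construction script does nothing.
; Disconnected nodes would cast the child actor to Chameleon and set the camera's world roll and pitch from clamped AngleX and AngleY while preserving yaw, but they never run.
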(event Custom|AngleVision)

(event EventBeginPlay
  (CallFunction|AngleVision))

(fn ConstructionScript)