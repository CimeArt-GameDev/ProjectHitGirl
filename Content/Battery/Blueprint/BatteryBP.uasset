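; BatteryBP is a battery pickup that the player collects by interacting with it.
; On BeginPlay it finds the ThirdPersonCharacter with GetActorOfClass and stores it as Player.
; InteractText prints a "Take" prompt, while InteractEvent prints confirmation, increments the player's BatteryNumber directly and destroys the battery.
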(event EventBeginPlay
  (bind _returnvalue (Actor|GetActorOfClass "/Game/ThirdPersonBP/Blueprints/ThirdPersonCharacter.ThirdPersonCharacter_C"))
  (Variables|Default|SetPlayer _returnvalue))

(event EventInteractText
  (Development|PrintString "Take"))

(event EventInteractEvent
  (bind _player (Variables|Default|GetPlayer))
  (Development|PrintString "Took")
  (Variables|/Game/ThirdPersonBP/Blueprints/ThirdPersonCharacter.ThirdPersonCharacter_C|SetBatteryNumber _player (+ (Variables|/Game/ThirdPersonBP/Blueprints/ThirdPersonCharacter.ThirdPersonCharacter_C|GetBatteryNumber _player) 1))
  (Actor|DestroyActor))

(fn ConstructionScript)