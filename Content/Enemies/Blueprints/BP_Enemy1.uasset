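; Enemy Blueprint that runs behavior tree BT_Enemy3 on BeginPlay and feeds it player detection through the Blackboard.
; AI Perception updates for BP_Player1 store the Player and set IsSeen, without checking whether the stimulus was gained or lost.
; A retriggerable delay clears IsSeen five seconds after the last such update.
; Tick prints IsSeen and RandomLocation on screen for debugging.
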(event OnTargetPerceptionUpdated(AIPerception)
  (params (Actor :type Actor%20Object%20Reference) (Stimulus :type AI%20Stimulus%20Structure))
  (bind _returnvalue (Utilities|Name|MakeLiteralName "IsSeen"))
  (bind _self self)
  (bind _returnvalue_2 (AI|GetBlackboard _self))
  ;[1 1 1] Set Value of Behavior "IsSeen"
  (bind _asbp_player_1 (Utilities|Casting|CastToBP_Player1 Actor))
  (AI|Components|Blackboard|SetValueasObject _returnvalue_2 (Utilities|Name|MakeLiteralName "Player") _asbp_player_1)
  (AI|Components|Blackboard|SetValueasBool _returnvalue_2 _returnvalue true)
  (Utilities|FlowControl|RetriggerableDelay 5.0)
  (AI|Components|Blackboard|SetValueasBool _returnvalue_2 _returnvalue false))

(event EventBeginPlay
  ;[1 1 1] Run Behavior
  (AI|RunBehaviorTree (AI|GetAIController self) "/Game/Enemies/IA/BT_Enemy3.BT_Enemy3"))

(event EventTick
  (params (DeltaSeconds :type Float%20%28single-precision%29))
  (bind _returnvalue (AI|GetBlackboard 0))
  ;[1 1 1] Debug
  (Development|PrintString (Utilities|String|Append "IsSeen: " (Utilities|String|ToString(Boolean) (ScalableFloat|GetValueasBool _returnvalue (Utilities|Name|MakeLiteralName "IsSeen"))) " 
" "Random Location: " (Utilities|String|ToString(Vector) (AI|Components|Blackboard|GetValueasVector _returnvalue (Utilities|Name|MakeLiteralName "RandomLocation")))) true true "(R=0.776042,G=0.025111,B=0.000000,A=1.000000)" 0.1))

(fn ConstructionScript)