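; BPC_Patrolling is an enemy AI component that supplies patrol destinations from an array of patrol point actors.
; FindNextPoint returns the location of the actor at the current index, then advances the index, wrapping to zero after the last entry so the route loops.
; BeginPlay and Tick are unused, so the component only does work when FindNextPoint is called.
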(event EventBeginPlay)

(event EventTick
  (params (DeltaSeconds :type Float%20%28single-precision%29)))

(fn FindNextPoint
  (LocalVariables|SetLocalPoint (Utilities|Array|Get(acopy) (Variables|Default|GetPatrollingPoints) (Variables|Default|GetCurrentPoint)))
  (Variables|Default|SetCurrentPoint (select (== (Variables|Default|GetCurrentPoint) (Utilities|Array|LastIndex (Variables|Default|GetPatrollingPoints))) 0 (+ (Variables|Default|GetCurrentPoint) 1)))
  (return (Transformation|GetActorLocation (LocalVariables|GetLocalPoint))))